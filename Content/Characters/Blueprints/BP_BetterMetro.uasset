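; BP_BetterMetro is a physics-driven actor that glides horizontally in a random direction, spinning and bouncing off whatever it hits, with a random hue on its duck material.
; Tick keeps capsule velocity horizontal and at least MaximumSpeed, easing excess speed down, while yawing the mesh.
; Hits on non-floor surfaces re-roll spin and play a scale-bounce timeline.
; Character hits also add a push-away impulse to avoid corner trapping.
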(event OnComponentHit(Capsule)
  (params (HitComponent :type Primitive%20Component%20Object%20Reference) (OtherActor :type Actor%20Object%20Reference) (OtherComp :type Primitive%20Component%20Object%20Reference) (NormalImpulse :type Vector :default "0, 0, 0") (Hit :type Hit%20Result%20Structure%20%28by%20ref%29))
  (bind _returnvalue (Transformation|GetActorLocation OtherActor))
  (bind _self self)
  (bind _returnvalue_2 (Transformation|GetActorLocation _self))
  (if (< (.z (Math|Vector|Normalize (.Normal (Collision|BreakHitResult Hit)))) 0.3)
    (CallFunction|SetNewRotationSpeed)
    (Utilities|FlowControl|Sequence
      (:then_0
        (bind _bounce (Timeline|Timeline PlayFromStart)
          (:Update
            (Transformation|SetRelativeScale3D (Variables|Default|GetSM_BettreMetro_body_low) (* _bounce (Variables|Default|GetStartingTempMeshScale))))))
      (:then_1
        ;[1 1 1] REBOUND ON PLAYER :D     (to avoid getting stuck in a corner lol)
        (if (Class|GameplayStatics|ObjectIsA OtherActor "/Script/Engine.Character")
          (Physics|AddImpulse (Variables|Default|GetCapsule) (* (Class|KismetMathLibrary|VectorNormal2D (- (Math|Vector|MakeVector (.x _returnvalue_2) (.y _returnvalue_2) 0.0) (Math|Vector|MakeVector (.x _returnvalue) (.y _returnvalue) 0.0)) 0.0001) (Variables|Default|GetPlayer%20Bounce%20Back%20Impulse%20Strength)) "None" true))))))

(event EventTick
  (params (DeltaSeconds :type Float%20%28single-precision%29))
  (CallFunction|SetSpeed DeltaSeconds)
  (Transformation|AddLocalRotation (Variables|Default|GetSM_BettreMetro_body_low) (Math|Rotator|MakeRotator 0.0 0.0 (* DeltaSeconds (Variables|Default|GetCurrent%20Rotation%20Speed))) false false))

(event EventBeginPlay
  ;[0.05098 0.05098 0.05098] Initialize
  (Variables|Default|SetStartingTempMeshScale (Variables|/Script/Engine.SceneComponent|GetRelativeScale3D (Variables|Default|GetSM_BettreMetro_body_low)))
  (bind _returnvalue (Rendering|Material|CreateDynamicMaterialInstance (Variables|Default|GetSM_BettreMetro_body_low) 1 "/Game/Materials/MI_Duck.MI_Duck" "None" :!class /Script/Engine.PrimitiveComponent))
  (Rendering|Material|SetScalarParameterValue _returnvalue "HueShift" (Math|Random|RandomFloat) :!class /Script/Engine.MaterialInstanceDynamic)
  (Physics|SetPhysicsLinearVelocity (Variables|Default|GetCapsule) (* (Class|KismetMathLibrary|VectorNormal2D (Math|Random|RandomUnitVector) 0.0001) (Variables|Default|GetMaximum%20Speed)) false "None")
  (CallFunction|SetNewRotationSpeed))

(fn ConstructionScript)

(fn SetSpeed
  (params (DeltaTime :type Float%20%28double-precision%29))
  (bind _returnvalue (Transformation|GetVelocity))
  (Physics|SetPhysicsLinearVelocity (Variables|Default|GetCapsule) (* (Math|Float|Max(Float) (Math|Interpolation|FInterpTo (Math|Vector|VectorLength _returnvalue) (Variables|Default|GetMaximum%20Speed) DeltaTime 1.0) (Variables|Default|GetMaximum%20Speed)) (Class|KismetMathLibrary|VectorNormal2D _returnvalue 0.0001)) false "None"))

(fn SetNewRotationSpeed
  (Variables|Default|SetCurrent%20Rotation%20Speed (Math|Random|RandomFloatinRange -3.6e+02 3.6e+02)))