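; BP_FlowerBouquetPot is an interactable pot that grows a flower bouquet and clears it on a later interaction.
; An interaction on an empty pot spawns a BP_FlowerBouquet at Plane2 with zero Z scale, and the FlowerGrow timeline stretches it vertically.
; Interacting once fully grown runs the parent interaction, destroys the bouquet and resets the pot.
; Interactions are ignored while growth is in progress.
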(event EventOnInteraction
  (params (Player :type Character%20Object%20Reference))
  (if (not (Variables|Default|GetIsInGrowing))
    (if (Variables|Default|GetIs%20grow)
      (|CallParentFunction Player)
      (Actor|DestroyActor (stale _returnvalue))
      (Variables|Default|SetIs%20grow false)
      (else
        (bind _returnvalue (Game|SpawnActorfromClass "/Game/Characters/Interaction/BP_FlowerBouquet.BP_FlowerBouquet_C" (Math|Transform|MakeTransform (Transformation|GetWorldLocation (Variables|Default|GetPlane2)) "0, 0, 0" "1.000000,1.000000,0.000000") "Undefined" "MultiplyWithRoot" 0 0))
        (bind _grow (Timeline|flower%20grow PlayFromStart)
          (:Update
            (Variables|Default|SetIsInGrowing true)
            (Transformation|SetActorScale3D _returnvalue (Math|Vector|MakeVector 1.0 1.0 _grow)))
          (:Finished
            (Variables|Default|SetIs%20grow true)
            (Variables|Default|SetIsInGrowing false)))))))

(fn ConstructionScript
  (|CallParentFunction))