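; BP_WaxBucket is an interactable wax bucket that disappears from the world on interaction and returns when dropped.
; OnInteraction runs the parent behavior, then hides the actor and disables its collision.
; OnDroped runs the parent behavior, then restores visibility and collision.
; Its CanInteract function always returns false.
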(event EventOnDroped
  (|CallParentFunction)
  ;[1 1 1] To Re-Enable
  (Rendering|SetActorHiddenInGame false)
  (Collision|SetActorEnableCollision true))

(event EventOnInteraction
  (params (Player :type Character%20Object%20Reference))
  (|CallParentFunction Player)
  (Rendering|SetActorHiddenInGame true)
  (Collision|SetActorEnableCollision false))

(fn ConstructionScript
  (|CallParentFunction))

(fn CanInteract
  (return false))