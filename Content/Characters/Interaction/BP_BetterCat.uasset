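; BP_BetterCat is a child interaction actor for a cat that disappears when interacted with and returns when dropped.
; On interaction it plays a door-opening 2D sound, runs the parent logic, then hides itself and disables collision.
; On drop it runs the parent logic, then restores visibility and collision.
; Its CanInteract function always returns false, and its construction script only calls the parent.
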(event EventOnDroped
  (|CallParentFunction)
  ;[1 1 1] To Re-Enable
  (Rendering|SetActorHiddenInGame false)
  (Collision|SetActorEnableCollision true))

(event EventOnInteraction
  (params (Player :type Character%20Object%20Reference))
  (Audio|PlaySound2D "/Game/sound/opening-the-front-door-210347.opening-the-front-door-210347" 1.0 1.0 0.0 0 0)
  (|CallParentFunction Player)
  (Rendering|SetActorHiddenInGame true)
  (Collision|SetActorEnableCollision false))

(fn ConstructionScript
  (|CallParentFunction))

(fn CanInteract
  (return false))