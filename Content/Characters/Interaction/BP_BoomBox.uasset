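; BP_BoomBox is an interactable boom box that plays audio and can be picked up and dropped.
; It extends a parent's interaction and drop events, calling the parent logic first.
; On interaction it hides the actor, disables collision and mutes the SonderAsphalt audio by volume multiplier rather than stopping it.
; On drop it restores visibility, collision and full volume.
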(event EventOnDroped
  (|CallParentFunction)
  ;[1 1 1] To Re-Enable
  (Rendering|SetActorHiddenInGame false)
  (Collision|SetActorEnableCollision true)
  (Audio|Components|Audio|SetVolumeMultiplier (Variables|Default|GetSonder-Asphalt) 1.0 :!class /Script/Engine.AudioComponent))

(event EventOnInteraction
  (params (Player :type Character%20Object%20Reference))
  (|CallParentFunction Player)
  (Rendering|SetActorHiddenInGame true)
  (Collision|SetActorEnableCollision false)
  (Audio|Components|Audio|SetVolumeMultiplier (Variables|Default|GetSonder-Asphalt) 0.0 :!class /Script/Engine.AudioComponent))

(fn ConstructionScript
  (|CallParentFunction))