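; Handheld water hose interactable that stays tethered by a cable to a fixed world-space end point.
; Each tick it pins the cable end there and sets cable length to 85% of the distance to keep it taut.
; While held, it follows the player's body rotation with a fixed offset; when dropped, it detaches, returns to its BeginPlay location and re-enables collision.
; A preview function displays the end point and updates cable length.
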(event EventBeginPlay
  (|CallParentFunction)
  (Variables|Default|SetBegin%20Play%20Location (Transformation|GetActorLocation)))

(event EventTick
  (params (DeltaSeconds :type Float%20%28single-precision%29))
  (Transformation|SetWorldLocationAndRotation (Variables|Default|GetCableEndPoint) (Variables|Default|GetWorld%20Space%20Cable%20End) "0, 0, 0" false false)
  (Variables|/Script/CableComponent.CableComponent|SetCableLength (Variables|Default|GetCable) (* (Math|Vector|Distance(Vector) (Transformation|GetActorLocation) (Variables|Default|GetWorld%20Space%20Cable%20End)) 0.85))
  (if (Variables|Default|GetCurrentlyHandled)
    (bind _body_rotation (Class|BPICharacter|GetBodyRotation(Message) (Variables|Default|GetPlayer) true))
    (Transformation|SetActorRotation (Math|Rotator|CombineRotators "0.000000,90.000000,0.000000" _body_rotation) true)))

(event EventOnHandled
  (|CallParentFunction))

(event EventOnDroped
  (|CallParentFunction)
  (Transformation|DetachFromActor "KeepWorld" "KeepWorld" "KeepWorld")
  (Transformation|SetActorLocationAndRotation (Variables|Default|GetBegin%20Play%20Location) "0, 0, 0")
  (Collision|SetActorEnableCollision true))

(event EventOnInteraction
  (params (Player :type Character%20Object%20Reference))
  (|CallParentFunction Player))

(fn ConstructionScript
  (|CallParentFunction))

(fn PreviewWorldSpace
  (CallFunction|DisplayLocation&Rotation (Variables|Default|GetWorld%20Space%20Cable%20End) "0, 0, 0" 1e+01 1e+01)
  (Variables|/Script/CableComponent.CableComponent|SetCableLength (Variables|Default|GetCable) (* (Math|Vector|Distance(Vector) (Transformation|GetActorLocation) (Variables|Default|GetWorld%20Space%20Cable%20End)) 0.85)))