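; BP_MasterOutlineManager controls a pulsing post-process outline that highlights the actor tied to a given machine need.
; BeginPlay puts a dynamic outline material instance on the level's PostProcessVolume, and Tick animates its width and glow with sine and cosine waves.
; SetNewOutline clears custom depth on all referenced actors' meshes, then enables it for the chosen need's actor, except for the first enum value.
; A helper rebuilds the need-to-actor map with empty entries.
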(event EventBeginPlay
  (bind _returnvalue (Rendering|Material|CreateDynamicMaterialInstance "/Game/Enviro/VFX/Materials/Outline/MI_Outline.MI_Outline" "None" "None" :!class /Script/Engine.KismetMaterialLibrary))
  (Variables|Default|SetOutline%20Material _returnvalue)
  (bind _returnvalue_2 (Actor|GetActorOfClass "/Script/Engine.PostProcessVolume"))
  (bind _structout (Utilities|Struct|SetmembersinPostProcessSettings (Variables|/Script/Engine.PostProcessVolume|GetSettings _returnvalue_2) (Utilities|Struct|MakeWeightedBlendables (Utilities|Array|MakeArray (Utilities|Struct|MakeWeightedBlendable 1.0 _returnvalue)))))
  (Variables|/Script/Engine.PostProcessVolume|SetSettings _returnvalue_2 _structout))

(event EventTick
  (params (DeltaSeconds :type Float%20%28single-precision%29))
  (bind _returnvalue (Actor|GetGameTimeSinceCreation))
  (bind _outline_material (Variables|Default|GetOutline%20Material))
  (Rendering|Material|SetScalarParameterValue _outline_material "Line Render Width" (+ (Math|Trig|Sin(Radians) (* _returnvalue (Variables|Default|GetSize%20Frequency))) 1.1) :!class /Script/Engine.MaterialInstanceDynamic)
  (Rendering|Material|SetScalarParameterValue _outline_material "Outline Glow Intensity" (+ (* (Math|Trig|Cos(Radians) (* _returnvalue (Variables|Default|GetGlow%20Frequency))) 0.4) 0.6) :!class /Script/Engine.MaterialInstanceDynamic))

(fn ConstructionScript)

(fn InitializeBecauseUnrealSucks
  (Utilities|Map|Clear (Variables|Default|GetReferences%20for%20each%20Needs))
  (bind _enumvalue (|ForEachEnum_MachineNeeds)
    (:LoopBody
      (Utilities|Map|Add (Variables|Default|GetReferences%20for%20each%20Needs) _enumvalue 0))))

(fn SetNewOutline
  (params (Key :type Enum_MachineNeeds%20Enum%20%28by%20ref%29 :default "NewEnumerator0"))
  (bind _values (Utilities|Map|Values (Variables|Default|GetReferences%20for%20each%20Needs)))
  (for _array_element _values
    (Utilities|IsValid _array_element
      (:Is%20Valid
        (for _array_element_2 (Actor|GetComponentsByClass _array_element "/Script/Engine.MeshComponent")
          (Rendering|SetRenderCustomDepth _array_element_2 false)))))
  (if (not (Utilities|Enum|Equal(Enum) Key (Utilities|Enum|LiteralenumEnum_MachineNeeds "NewEnumerator0")))
    (bind _output_get (LocalVariables|SetActorToAct (.Value (Utilities|Map|Find (Variables|Default|GetReferences%20for%20each%20Needs) Key))))
    (for _array_element_3 (Actor|GetComponentsByClass _output_get "/Script/Engine.MeshComponent")
      (Rendering|SetRenderCustomDepth _array_element_3 true))))