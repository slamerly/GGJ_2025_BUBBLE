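; Animated pipe prop that pumps at random while idle and runs a pipe sequence to trigger the spawn machine.
; SpawnObject and AnimationSpawn start chained timelines that end by messaging the first BPI_SpawnMachine actor found at BeginPlay.
; A self-restarting loop waits a random delay, then plays one of four pump timelines.
; All timelines animate through scalars in a Material Parameter Collection, with rattle and bang sounds at hardcoded world locations.
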(event Custom|SpawnObject
  (bind _alpha (Timeline|Timeline_2 Play)
    (:Update
      (Rendering|Material|SetScalarParameterValue "/Game/MaterialParameterCollection.MaterialParameterCollection" "Time_E" _alpha :!class /Script/Engine.KismetMaterialLibrary))
    (:Finished
      (Utilities|FlowControl|Sequence
        (:then_0
          (bind _alpha_2 (Timeline|Timeline_3 PlayFromStart)
            (:Update
              (Rendering|Material|SetScalarParameterValue "/Game/MaterialParameterCollection.MaterialParameterCollection" "Time_F" _alpha_2 :!class /Script/Engine.KismetMaterialLibrary))
            (:Finished
              (Utilities|FlowControl|Sequence
                (:then_0
                  (bind _alpha_3 (Timeline|Timeline_0 Play)
                    (:Update
                      (Rendering|Material|SetScalarParameterValue "/Game/MaterialParameterCollection.MaterialParameterCollection" "Time_C" _alpha_3 :!class /Script/Engine.KismetMaterialLibrary))
                    (:Finished
                      (Class|BPISpawnMachine|MachineAnimationSpawn(Message) (Variables|Default|GetSpawnMachine)))))
                (:then_1
                  (Audio|PlaySoundatLocation "/Game/sound/Ambiant/ggj_water_pipe_a.ggj_water_pipe_a" "400.000000,-550.000000,94.000000" "0, 0, 0" 0.5 0.8 0.0 0 0 0 0)
                  (Audio|PlaySoundatLocation "/Game/sound/Ambiant/ggj_ambiant_rattling.ggj_ambiant_rattling" "400.000000,-550.000000,94.000000" "0, 0, 0" 0.5 0.8 0.0 0 0 0 0)
                  (Utilities|FlowControl|Delay 0.23)
                  (Audio|PlaySoundatLocation "/Game/sound/Ambiant/ggj_metalbang.ggj_metalbang" "400.000000,-550.000000,93.000000" "0, 0, 0" 0.7 1.5 0.0 0 0 0 0))))))
        (:then_1
          (Audio|PlaySoundatLocation "/Game/sound/Ambiant/ggj_water_pipe_a.ggj_water_pipe_a" "-828.000000,-304.000000,94.000000" "0, 0, 0" 0.5 1.0 0.0 0 0 0 0)
          (Utilities|FlowControl|Delay 0.5)
          (Audio|PlaySoundatLocation "/Game/sound/Ambiant/ggj_metalbang_b.ggj_metalbang_b" "-828.000000,-304.000000,94.000000" "0, 0, 0" 0.5 1.0 0.0 0 0 0 0))))))

(event Custom|RandomAnim
  (Utilities|FlowControl|Delay (Math|Random|RandomFloatinRange 0.0 (Variables|Default|GetMaxDurationBetweenRandomAnimation)))
  (switch int (Math|Random|RandomIntegerinRange 0 3)
    (:0
      (CallFunction|PumpPipeA))
    (:1
      (CallFunction|PumpPipeB))
    (:2
      (CallFunction|PumpPipeC))
    (:3
      (CallFunction|PumpPipeD))))

(event Custom|PumpPipeA
  (bind _alpha (Timeline|Timeline PlayFromStart)
    (:Update
      (Rendering|Material|SetScalarParameterValue "/Game/MaterialParameterCollection.MaterialParameterCollection" "Time_B" _alpha :!class /Script/Engine.KismetMaterialLibrary))
    (:Finished
      (CallFunction|RandomAnim)
      (Audio|PlaySoundatLocation "/Game/sound/Ambiant/ggj_water_pipe_b.ggj_water_pipe_b" "347.372618,781.622735,526.644744" "0, 0, 0" 0.5 1.0 0.0 0 0 0 0))))

(event Custom|PumpPipeB
  (bind _alpha (Timeline|Timeline_1 PlayFromStart)
    (:Update
      (Rendering|Material|SetScalarParameterValue "/Game/MaterialParameterCollection.MaterialParameterCollection" "Time_D" _alpha :!class /Script/Engine.KismetMaterialLibrary))
    (:Finished
      (CallFunction|RandomAnim)
      (Audio|PlaySoundatLocation "/Game/sound/Ambiant/ggj_water_pipe_a.ggj_water_pipe_a" "347.372618,781.622735,526.644744" "0, 0, 0" 0.7 0.8 0.0 0 0 0 0)
      (Audio|PlaySoundatLocation "/Game/sound/Ambiant/ggj_metalbang_b.ggj_metalbang_b" "-828.000000,-304.000000,94.000000" "0, 0, 0" 0.4 1.0 0.0 0 0 0 0))))

(event Custom|PumpPipeC
  (bind _alpha (Timeline|Timeline_4 PlayFromStart)
    (:Update
      (Rendering|Material|SetScalarParameterValue "/Game/MaterialParameterCollection.MaterialParameterCollection" "Time_G" _alpha :!class /Script/Engine.KismetMaterialLibrary))
    (:Finished
      (CallFunction|RandomAnim)
      (Audio|PlaySoundatLocation "/Game/sound/Ambiant/ggj_water_pipe_a.ggj_water_pipe_a" "400.000000,-550.000000,94.000000" "0, 0, 0" 0.7 0.8 0.0 0 0 0 0)
      (Audio|PlaySoundatLocation "/Game/sound/Ambiant/ggj_ambiant_rattling.ggj_ambiant_rattling" "400.000000,-550.000000,94.000000" "0, 0, 0" 0.5 0.8 0.0 0 0 0 0))))

(event Custom|PumpPipeD
  (bind _alpha (Timeline|Timeline_5 PlayFromStart)
    (:Update
      (Rendering|Material|SetScalarParameterValue "/Game/MaterialParameterCollection.MaterialParameterCollection" "Time_A" _alpha :!class /Script/Engine.KismetMaterialLibrary))
    (:Finished
      (CallFunction|RandomAnim)
      (Audio|PlaySoundatLocation "/Game/sound/Ambiant/ggj_water_pipe_b.ggj_water_pipe_b" "400.000000,-550.000000,94.000000" "0, 0, 0" 0.7 1.2 0.0 0 0 0 0)
      (Audio|PlaySoundatLocation "/Game/sound/Ambiant/ggj_metalbang.ggj_metalbang" "-828.000000,-304.000000,94.000000" "0, 0, 0" 0.4 1.0 0.0 0 0 0 0))))

(event EventBeginPlay
  (bind _outactors (Actor|GetAllActorswithInterface "/Game/Enviro/BP/BPI_SpawnMachine.BPI_SpawnMachine_C"))
  (Variables|Default|SetSpawnMachine (Utilities|Array|Get(acopy) _outactors))
  (CallFunction|RandomAnim))

(event EventAnimationSpawn
  (Utilities|FlowControl|Sequence
    (:then_0
      (bind _alpha (Timeline|Timeline_2 PlayFromStart)
        (:Update
          (Rendering|Material|SetScalarParameterValue "/Game/MaterialParameterCollection.MaterialParameterCollection" "Time_E" _alpha :!class /Script/Engine.KismetMaterialLibrary))
        (:Finished
          (Utilities|FlowControl|Sequence
            (:then_0
              (bind _alpha_2 (Timeline|Timeline_3 PlayFromStart)
                (:Update
                  (Rendering|Material|SetScalarParameterValue "/Game/MaterialParameterCollection.MaterialParameterCollection" "Time_F" _alpha_2 :!class /Script/Engine.KismetMaterialLibrary))
                (:Finished
                  (Utilities|FlowControl|Sequence
                    (:then_0
                      (bind _alpha_3 (Timeline|Timeline_0 Play)
                        (:Update
                          (Rendering|Material|SetScalarParameterValue "/Game/MaterialParameterCollection.MaterialParameterCollection" "Time_C" _alpha_3 :!class /Script/Engine.KismetMaterialLibrary))
                        (:Finished
                          (Class|BPISpawnMachine|MachineAnimationSpawn(Message) (Variables|Default|GetSpawnMachine)))))
                    (:then_1
                      (Audio|PlaySoundatLocation "/Game/sound/Ambiant/ggj_water_pipe_a.ggj_water_pipe_a" "400.000000,-550.000000,94.000000" "0, 0, 0" 0.5 0.8 0.0 0 0 0 0)
                      (Audio|PlaySoundatLocation "/Game/sound/Ambiant/ggj_ambiant_rattling.ggj_ambiant_rattling" "400.000000,-550.000000,94.000000" "0, 0, 0" 0.5 0.8 0.0 0 0 0 0)
                      (Utilities|FlowControl|Delay 0.23)
                      (Audio|PlaySoundatLocation "/Game/sound/Ambiant/ggj_metalbang.ggj_metalbang" "400.000000,-550.000000,93.000000" "0, 0, 0" 0.7 1.5 0.0 0 0 0 0))))))
            (:then_1
              (Audio|PlaySoundatLocation "/Game/sound/Ambiant/ggj_water_pipe_a.ggj_water_pipe_a" "-828.000000,-304.000000,94.000000" "0, 0, 0" 0.5 1.0 0.0 0 0 0 0)
              (Utilities|FlowControl|Delay 0.5)
              (Audio|PlaySoundatLocation "/Game/sound/Ambiant/ggj_metalbang_b.ggj_metalbang_b" "-828.000000,-304.000000,94.000000" "0, 0, 0" 0.5 1.0 0.0 0 0 0 0))))))
    (:then_1
      (Audio|PlaySoundatLocation "/Game/sound/Ambiant/ggj_water_pipe_b.ggj_water_pipe_b" "347.372618,781.622735,526.644744" "0, 0, 0" 0.5 1.0 0.0 0 0 0 0)
      (Audio|PlaySoundatLocation "/Game/sound/Ambiant/ggj_ambiant_rattling.ggj_ambiant_rattling" "347.372618,781.622735,526.644744" "0, 0, 0" 0.5 1.0 0.0 0 0 0 0)
      (Utilities|FlowControl|Delay 0.5)
      (Audio|PlaySoundatLocation "/Game/sound/Ambiant/ggj_metalbang.ggj_metalbang" "347.372618,781.622735,526.644744" "0, 0, 0" 0.5 1.0 0.0 0 0 0 0))))

(fn ConstructionScript)