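; Machine dispenser that drops a random machine from an arrow point on BeginPlay and later swaps it through a lever-operated trap.
; Timelines animate each step: lever pull, trap opening, old machine falling and being destroyed, trap closing, lever return, then a new spawn.
; OnInteraction starts the cycle behind lever and CleanIsFinish flags; MachineSatisphied starts it directly.
; Several timelines start from another's Update output rather than Finished.
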(event Custom|SpawnANewMachine
  (bind _machinetospawn (Variables|Default|GetMachineToSpawn))
  (bind _arrow (Variables|Default|GetArrow))
  (bind _returnvalue (Transformation|GetWorldLocation _arrow))
  ;[0.4664 1 0.6562] Spawn a radom machine
  (if (Variables|Default|GetCanSpawnNew)
    (Variables|Default|SetCanSpawnNew false)
    (bind _returnvalue_2 (Game|SpawnActorfromClass (Utilities|Array|Get(acopy) _machinetospawn (Math|Random|RandomInteger (Utilities|Array|Length _machinetospawn))) (Math|Transform|MakeTransform (Transformation|GetWorldLocation (Variables|Default|GetArrow)) (Transformation|GetActorRotation) "1.000000,1.000000,1.000000") "AlwaysSpawn" "MultiplyWithRoot" 0 0))
    (bind _output_get (Variables|Default|SetMachineFalling _returnvalue_2))
    (bind _falling (Timeline|Fall PlayFromStart)
      (:Update
        (Transformation|SetActorRelativeLocation _output_get (Math|Vector|MakeVector (.x _returnvalue) (.y _returnvalue) (- (.z (Variables|/Script/Engine.SceneComponent|GetRelativeLocation _arrow)) _falling))))
      (:Finished
        (Variables|Default|SetMachineToClean _output_get)
        (Variables|Default|SetCanSpawnNew true)))))

(event EventOnInteraction
  (params (Player :type Character%20Object%20Reference))
  (bind _arrow (Variables|Default|GetArrow))
  (bind _sphere (Variables|Default|GetSphere))
  (bind _machinetoclean (Variables|Default|GetMachineToClean))
  (bind _returnvalue (Transformation|GetWorldLocation _arrow))
  (bind _relativerotation (Variables|/Script/Engine.SceneComponent|GetRelativeRotation _sphere))
  (if (Variables|Default|GetCanActiveLeverAgin)
    (Variables|Default|SetCanActiveLeverAgin false)
    (if (Variables|Default|GetClean%20is%20finish%20)
      (Variables|Default|SetClean%20is%20finish%20 false)
      ;[1 1 1] Move Lever
      (Variables|Default|SetRelative%20Rotation%20Y%20%28Pitch%29 (.pitch _relativerotation))
      (bind _newtrack_1 (Timeline|Timeline_0 Play)
        (:Update
          (Transformation|SetRelativeRotation _sphere (Math|Rotator|MakeRotator 0.0 (- (Variables|Default|GetRelative%20Rotation%20Y%20%28Pitch%29) _newtrack_1) 0.0) false false))
        (:Finished
          (Variables|Default|SetRelative%20Rotation%20Y%20%28Pitch%29 (.pitch _relativerotation))
          ;[1 1 1] Trap Open
          (bind _newtrack_1_2 (Timeline|Timeline_2 PlayFromStart)
            (:Update
              (Transformation|SetRelativeRotation (Variables|Default|GetTrapPivot) (Math|Rotator|MakeRotator _newtrack_1_2 0.0 0.0) false false)
              ;[1 1 1] Machine fall
              (bind _falling (Timeline|Timeline PlayFromStart)
                (:Update
                  (Transformation|SetActorRelativeLocation _machinetoclean (Math|Vector|MakeVector (.x _returnvalue) (.y _returnvalue) (- (.z (Transformation|GetWorldLocation (Variables|Default|GetTrap))) _falling))))
                (:Finished
                  (Actor|DestroyActor _machinetoclean)
                  ;[1 1 1] Trap close
                  (bind _newtrack_1_3 (Timeline|Timeline_3 PlayFromStart)
                    (:Update
                      (Transformation|SetRelativeRotation (Variables|Default|GetTrapPivot) (Math|Rotator|MakeRotator _newtrack_1_3 0.0 0.0) false false)
                      ;[1 1 1] lever reverse
                      (bind _newtrack_1_4 (Timeline|Timeline_1 Play)
                        (:Update
                          (Transformation|SetRelativeRotation (Variables|Default|GetSphere) (Math|Rotator|MakeRotator 0.0 (+ _newtrack_1_4 (Variables|Default|GetRelative%20Rotation%20Y%20%28Pitch%29)) 0.0) false false))
                        (:Finished
                          (CallFunction|SpawnANewMachine)
                          (Variables|Default|SetCanActiveLeverAgin true)
                          (Variables|Default|SetClean%20is%20finish%20 false)))))))))))
      (else
        (Development|PrintString "je suis faux")))))

(event EventMachineSatisphied
  (bind _arrow (Variables|Default|GetArrow))
  (bind _sphere (Variables|Default|GetSphere))
  (bind _machinetoclean (Variables|Default|GetMachineToClean))
  (bind _returnvalue (Transformation|GetWorldLocation _arrow))
  (bind _relativerotation (Variables|/Script/Engine.SceneComponent|GetRelativeRotation _sphere))
  (Development|PrintString "animation")
  ;[1 1 1] Move Lever
  (Variables|Default|SetRelative%20Rotation%20Y%20%28Pitch%29 (.pitch _relativerotation))
  (bind _newtrack_1 (Timeline|Timeline_0 Play)
    (:Update
      (Transformation|SetRelativeRotation _sphere (Math|Rotator|MakeRotator 0.0 (- (Variables|Default|GetRelative%20Rotation%20Y%20%28Pitch%29) _newtrack_1) 0.0) false false))
    (:Finished
      (Variables|Default|SetRelative%20Rotation%20Y%20%28Pitch%29 (.pitch _relativerotation))
      ;[1 1 1] Trap Open
      (bind _newtrack_1_2 (Timeline|Timeline_2 PlayFromStart)
        (:Update
          (Transformation|SetRelativeRotation (Variables|Default|GetTrapPivot) (Math|Rotator|MakeRotator _newtrack_1_2 0.0 0.0) false false)
          ;[1 1 1] Machine fall
          (bind _falling (Timeline|Timeline PlayFromStart)
            (:Update
              (Transformation|SetActorRelativeLocation _machinetoclean (Math|Vector|MakeVector (.x _returnvalue) (.y _returnvalue) (- (.z (Transformation|GetWorldLocation (Variables|Default|GetTrap))) _falling))))
            (:Finished
              (Actor|DestroyActor _machinetoclean)
              ;[1 1 1] Trap close
              (bind _newtrack_1_3 (Timeline|Timeline_3 PlayFromStart)
                (:Update
                  (Transformation|SetRelativeRotation (Variables|Default|GetTrapPivot) (Math|Rotator|MakeRotator _newtrack_1_3 0.0 0.0) false false)
                  ;[1 1 1] lever reverse
                  (bind _newtrack_1_4 (Timeline|Timeline_1 Play)
                    (:Update
                      (Transformation|SetRelativeRotation (Variables|Default|GetSphere) (Math|Rotator|MakeRotator 0.0 (+ _newtrack_1_4 (Variables|Default|GetRelative%20Rotation%20Y%20%28Pitch%29)) 0.0) false false))
                    (:Finished
                      (CallFunction|SpawnANewMachine)
                      (Variables|Default|SetCanActiveLeverAgin true)
                      (Variables|Default|SetClean%20is%20finish%20 false))))))))))))

(event EventBeginPlay
  (bind _machinetospawn (Variables|Default|GetMachineToSpawn))
  (bind _arrow (Variables|Default|GetArrow))
  (bind _returnvalue (Transformation|GetWorldLocation _arrow))
  ;[0.4664 1 0.6562] Spawn a radom machine
  (if (Variables|Default|GetCanSpawnNew)
    (Variables|Default|SetCanSpawnNew false)
    (bind _returnvalue_2 (Game|SpawnActorfromClass (Utilities|Array|Get(acopy) _machinetospawn (Math|Random|RandomInteger (Utilities|Array|Length _machinetospawn))) (Math|Transform|MakeTransform (Transformation|GetWorldLocation (Variables|Default|GetArrow)) (Transformation|GetActorRotation) "1.000000,1.000000,1.000000") "AlwaysSpawn" "MultiplyWithRoot" 0 0))
    (bind _output_get (Variables|Default|SetMachineFalling _returnvalue_2))
    (bind _falling (Timeline|Fall PlayFromStart)
      (:Update
        (Transformation|SetActorRelativeLocation _output_get (Math|Vector|MakeVector (.x _returnvalue) (.y _returnvalue) (- (.z (Variables|/Script/Engine.SceneComponent|GetRelativeLocation _arrow)) _falling))))
      (:Finished
        (Variables|Default|SetMachineToClean _output_get)
        (Variables|Default|SetCanSpawnNew true)))))

(fn ConstructionScript)