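; BP_Machine is a needy machine with a random mesh and a list of random requests, shown on a camera-facing plane and through the outline manager.
; Handing it the requested item spawns a matching cosmetic effect and advances the list; a wrong item temporarily changes the countdown rate.
; The countdown is a timeline moving sparks along a spline cable.
; Completing the list or running out of time reports to EndGame, then notifies the spawner after a delay.
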(event Custom|CallNextMachine
  (Utilities|FlowControl|Delay (Variables|Finality|GetDelayBeforeNewSpawn))
  (Class|BPISpawnMachine|MachineSatisphied(Message) (Variables|Default|GetSpawner))
  (Components|DestroyComponent (Variables|Default|GetSparks)))

(event Custom|TimerMalus
  (Components|Timeline|SetPlayRate (Variables|Default|GetT_Sparks) (/ 1.0 (/ (Variables|Default|GetTimer) (Variables|Penality|GetDivideMalus))))
  (Utilities|FlowControl|Delay (Variables|Penality|GetDurationMalus))
  (Components|Timeline|SetPlayRate (Variables|Default|GetT_Sparks) (/ 1.0 (Variables|Default|GetTimer))))

(event EventOntheFloor
  (bind _spline (Variables|Default|Getspline))
  (Components|Timeline|SetPlayRate (Variables|Default|GetT_Sparks) (/ 1.0 (Variables|Default|GetTimer)))
  (bind _returnvalue (Niagara|SpawnSystematLocation "/Game/Enviro/VFX/NS_Sparks.NS_Sparks" "0, 0, 0"))
  (bind _output_get (Variables|Default|SetSparks _returnvalue))
  (Niagara|SetNiagaraVariable(Float) _output_get "Sphere Size" 4e+01)
  (bind _newtrack_0 (Timeline|T_Sparks PlayFromStart)
    (:Update
      (Transformation|SetWorldLocationAndRotation (Variables|Default|GetSparks) (Spline|GetLocationatDistanceAlongSpline _spline (Math|Float|Lerp 0.0 (Spline|GetSplineLength _spline) _newtrack_0) "World") (Spline|GetRotationatDistanceAlongSpline _spline (Math|Float|Lerp 0.0 (Spline|GetSplineLength _spline) _newtrack_0) "World") false false))
    (:Finished
      (Finality|Unsatisfied))))

(event EventTick
  (params (DeltaSeconds :type Float%20%28single-precision%29))
  (bind _plane (Variables|Default|GetPlane))
  (Transformation|SetWorldRotation _plane (Math|Rotator|MakeRotfromZY (- (Camera|GetCameraLocation (Variables|Default|GetPlayer%20Camera%20Manager)) (Transformation|GetWorldLocation _plane)) (Math|Vector|MakeVector 0.0 0.0 -1.0)) false false))

(event EventOnInteraction
  (params (Player :type Character%20Object%20Reference))
  (bind _currentplayerhandle (Class|BPICharacter|GetHandle(Message) Player))
  (if (Utilities|Enum|NotEqual(Enum) _currentplayerhandle "NewEnumerator0")
    (bind _match (Request|CorrespondRequest _currentplayerhandle))
    (Class|BPICharacter|DestroyHandle(Message) (Variables|Default|GetPlayer))
    (Default|OnEndOverlapOwner (Variables|Default|GetBPAC_Interactable) 0 (Variables|Default|GetPlayer))
    (if _match
      (Request|NextRequest)
      (else
        (Finality|Penality)))))

(event EventBeginPlay
  (bind _returnvalue (Game|GetPlayerCharacter 0))
  (CallFunction|VisualChange)
  (bind _returnvalue_2 (Actor|GetActorOfClass "/Game/Characters/Interaction/BP_MasterOutlineManager.BP_MasterOutlineManager_C"))
  (Variables|Default|SetOutline%20Manager _returnvalue_2)
  (if (Utilities|DoesObjectImplementInterface _returnvalue "/Game/Characters/Blueprints/BPI_Character.BPI_Character_C")
    (Variables|Default|SetPlayer _returnvalue)
    (bind _outactors (Actor|GetAllActorswithInterface "/Game/Enviro/BP/BPI_SpawnMachine.BPI_SpawnMachine_C"))
    (Variables|Default|SetSpawner (Utilities|Array|Get(acopy) _outactors))
    (Request|GenerationRequest (Variables|Request|GetNb%20Requests))
    (Request|SetRequest)
    (Variables|Default|SetPlayer%20Camera%20Manager (Game|GetPlayerCameraManager 0))
    (bind _returnvalue_3 (Actor|GetActorOfClass "/Game/HoudiniEngine/Bake/BP_SplineCable.BP_SplineCable_C"))
    (bind _output_get (Variables|Default|SetCable _returnvalue_3))
    (Variables|Default|Setspline (Actor|GetComponentbyClass _output_get "/Script/Engine.SplineComponent"))
    (bind _outactors_2 (Actor|GetAllActorswithInterface "/Game/Enviro/BP/BPI_EndGame.BPI_EndGame_C"))
    (Variables|Default|SetEndGame (Utilities|Array|Get(acopy) _outactors_2))))

(fn ConstructionScript)

(fn SetRequest
  (bind _currentrequest (Variables|Request|GetCurrentRequest))
  (bind _requestlist (Variables|Request|GetRequestList))
  (bind _output (Utilities|Array|Get(acopy) _requestlist _currentrequest))
  (Default|SetNewOutline (Variables|Default|GetOutline%20Manager) _output)
  (Rendering|Material|SetMaterial (Variables|Default|GetPlane) 0 (.Value (Utilities|Map|Find (Variables|Default|GetMaterial) _output))))

(fn GenerationRequest
  (params (NbRequests :type Integer))
  (for _index (range 0 (- NbRequests 1))
    (bind _output_get (LocalVariables|SetRandomRequest (Math|Random|RandomIntegerinRange 1 (- (|GetNumEnumEntries) 1))))
    (Utilities|Array|AddUnique (Variables|Request|GetRequestList) (Utilities|Enum|ByteToEnumEnum_MachineNeeds (Math|Conversions|ToByte(Integer) _output_get)))))

(fn CorrespondRequest
  (params (PlayerHandle :type Enum_ObjectHandled%20Enum :default "NewEnumerator0"))
  (bind _returnvalue (Transformation|GetActorLocation))
  (bind _staticmesh (Variables|Default|GetStaticMesh))
  (bind _staticmesh_2 (Variables|Default|GetStaticMesh))
  (bind _staticmesh_3 (Variables|Default|GetStaticMesh))
  (bind _staticmesh_4 (Variables|Default|GetStaticMesh))
  (bind _returnvalue_2 (Transformation|GetSocketTransform _staticmesh_2 "CHAMP" "RTS_World"))
  (bind _returnvalue_3 (Transformation|GetSocketTransform _staticmesh_3 "CAT" "RTS_World"))
  (bind _returnvalue_4 (Transformation|GetSocketTransform _staticmesh_4 "BOW" "RTS_World"))
  (bind _returnvalue_5 (Transformation|GetSocketTransform _staticmesh "FLOWER" "RTS_World"))
  (if (== (Math|Conversions|ToInteger(Byte) PlayerHandle) (Math|Conversions|ToInteger(Byte) (Utilities|Array|Get(acopy) (Variables|Request|GetRequestList) (Variables|Request|GetCurrentRequest))))
    (Utilities|FlowControl|Sequence
      (:then_0
        (switch Utilities|FlowControl|Switch|SwitchonEnum_ObjectHandled PlayerHandle
          (:NewEnumerator1
            ;[1 1 1] CHAT
            (bind _returnvalue_6 (Game|SpawnActorfromClass "/Game/Characters/Interaction/BP_Cat.BP_Cat_C" (Math|Transform|MakeTransform (.location _returnvalue_3) (.rotation _returnvalue_3) "1.000000,1.000000,1.000000") "Undefined" "MultiplyWithRoot" 0 0))
            (Transformation|AttachComponentToComponent _returnvalue_6 _staticmesh_3 "CAT" "KeepWorld" "KeepWorld" "KeepWorld" true))
          (:NewEnumerator2
            ;[1 1 1] Spawn Pentagram
            (bind _returnvalue_7 (Game|SpawnActorfromClass "/Script/Engine.DecalActor" (Math|Transform|MakeTransform "0.000000,-100.000000,0.000000" "-90.000000,0.000000,0.000000" "0.100000,1.000000,1.000000") "AlwaysSpawn" "OverrideRootScale" 0 0))
            (Rendering|Components|Decal|SetDecalMaterial (Variables|/Script/Engine.DecalActor|GetDecal _returnvalue_7) "/Game/Materials/MI_Decal.MI_Decal")
            (Rendering|Components|Decal|SetFadeOut (Variables|/Script/Engine.DecalActor|GetDecal _returnvalue_7) 8.0 5.0 true))
          (:NewEnumerator3
            ;[1 1 1] CHAT
            (bind _returnvalue_8 (Game|SpawnActorfromClass "/Game/Characters/Interaction/BP_FlowerBouquet.BP_FlowerBouquet_C" (Math|Transform|MakeTransform (.location _returnvalue_5) (.rotation _returnvalue_5) "1.000000,1.000000,1.000000") "Undefined" "MultiplyWithRoot" 0 0))
            (Transformation|AttachComponentToComponent _returnvalue_8 _staticmesh "FLOWER" "KeepWorld" "KeepWorld" "KeepWorld" true))
          (:NewEnumerator4
            ;[1 1 1] Spawn & Remove clean soap bubbles
            (bind _returnvalue_9 (Niagara|SpawnSystematLocation "/Game/Enviro/VFX/NS_Bubbles_Trail.NS_Bubbles_Trail" (Transformation|GetActorLocation)))
            (Variables|Default|SetClean%20Bubble%20Niagara _returnvalue_9))
          (:NewEnumerator5
            (bind _clean_bubble_niagara (Variables|Default|GetClean%20Bubble%20Niagara)
              (:then
                (Components|DestroyComponent _clean_bubble_niagara))
              (:else)))
          (:NewEnumerator6
            ;[1 1 1] DIco
            (bind _returnvalue_10 (Game|SpawnActorfromClass "/Game/Characters/Interaction/BP_DiscoGlitter.BP_DiscoGlitter_C" (Math|Transform|MakeTransform (Math|Vector|MakeVector (.x _returnvalue) (.y _returnvalue) (+ (.z _returnvalue) 5e+02)) "0, 0, 0" "1.000000,1.000000,1.000000") "Undefined" "MultiplyWithRoot" 0 0))
            (Actor|SetLifeSpan _returnvalue_10 2.0))
          (:NewEnumerator7
            ;[1 1 1] Tag
            (bind _returnvalue_11 (Game|SpawnActorfromClass "/Script/Engine.DecalActor" (Math|Transform|MakeTransform "0.000000,-100.000000,0.000000" "-90.000000,0.000000,0.000000" "0.100000,1.000000,1.000000") "AlwaysSpawn" "OverrideRootScale" 0 0))
            (Rendering|Components|Decal|SetDecalMaterial (Variables|/Script/Engine.DecalActor|GetDecal _returnvalue_11) (.OutItem (Utilities|Array|Random (LocalVariables|GetMI_DecalTag))))
            (Rendering|Components|Decal|SetFadeOut (Variables|/Script/Engine.DecalActor|GetDecal _returnvalue_11) 8.0 5.0 true))
          (:NewEnumerator8
            ;[1 1 1] BOW
            (bind _returnvalue_12 (Game|SpawnActorfromClass "/Game/Characters/Interaction/BP_BowTie.BP_BowTie_C" (Math|Transform|MakeTransform (.location _returnvalue_4) (.rotation _returnvalue_4) "1.000000,1.000000,1.000000") "Undefined" "MultiplyWithRoot" 0 0))
            (Transformation|AttachComponentToComponent _returnvalue_12 _staticmesh_4 "BOW" "KeepWorld" "KeepWorld" "KeepWorld" true))
          (:NewEnumerator9
            ;[1 1 1] CHAMPAGNE
            (bind _returnvalue_13 (Game|SpawnActorfromClass "/Game/Characters/Interaction/BP_CHAMP.BP_CHAMP_C" (Math|Transform|MakeTransform (.location _returnvalue_2) (.rotation _returnvalue_2) "1.000000,1.000000,1.000000") "Undefined" "MultiplyWithRoot" 0 0))
            (Transformation|AttachComponentToComponent _returnvalue_13 _staticmesh_2 "CHAMP" "KeepWorld" "KeepWorld" "KeepWorld" true))
          (:NewEnumerator14
            ;[1 1 1] WAX
            (Game|SpawnActorfromClass "/Game/Characters/Interaction/BP_WaxPouring.BP_WaxPouring_C" (Math|Transform|MakeTransform "150.000000,0.000000,300.000000" "0, 0, 0" "1.000000,1.000000,1.000000") "Undefined" "MultiplyWithRoot" 0 0))
          (:NewEnumerator15
            (Game|SpawnActorfromClass "/Game/Characters/Interaction/BP_BoomMusic.BP_BoomMusic_C" (Math|Transform|MakeTransform "150.000000,0.000000,300.000000" "0, 0, 0" "1.000000,1.000000,1.000000") "Undefined" "MultiplyWithRoot" 0 0))))
      (:then_1
        (return true)))
    (else
      (return false))))

(fn NextRequest
  (bind _result (Math|Integer|IncrementInt (Variables|Request|GetCurrentRequest))
    (:%20%20
      (if (>= _result (Utilities|Array|Length (Variables|Request|GetRequestList)))
        (Finality|Satisfied)
        (else
          (Request|SetRequest))))))

(fn Satisfied
  (Class|BPIEndGame|IncreaseSatisfied(Message) (Variables|Default|GetEndGame))
  (CallFunction|CallNextMachine)
  (bind _clean_bubble_niagara (Variables|Default|GetClean%20Bubble%20Niagara)
    (:then
      (Components|DestroyComponent _clean_bubble_niagara))
    (:else)))

(fn Penality
  (CallFunction|TimerMalus))

(fn VisualChange
  (bind _staticmesh (Variables|Default|GetStaticMesh))
  (bind _new_mesh (Variables|Default|GetNew%20Mesh))
  (bind _output_get (LocalVariables|SetIndex (Math|Random|RandomIntegerinRange 0 (- (Utilities|Map|Length _new_mesh) 1))))
  (bind _keys (Utilities|Map|Keys _new_mesh))
  (Components|StaticMesh|SetStaticMesh _staticmesh (Utilities|Array|Get(acopy) _keys _output_get))
  (bind _values (Utilities|Map|Values _new_mesh))
  (Transformation|SetRelativeScale3D _staticmesh (Utilities|Array|Get(acopy) _values _output_get)))

(fn Unsatisfied
  (Class|BPIEndGame|IncreaseUnsatisfied(Message) (Variables|Default|GetEndGame))
  (CallFunction|CallNextMachine)
  (bind _clean_bubble_niagara (Variables|Default|GetClean%20Bubble%20Niagara)
    (:then
      (Components|DestroyComponent _clean_bubble_niagara))
    (:else)))