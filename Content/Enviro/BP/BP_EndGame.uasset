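; End-of-game manager actor that runs the match countdown and tallies satisfied and unsatisfied counts.
; BeginPlay creates the WBP_EndGame widget, and Tick decrements the timer by one per frame, independent of delta time, to update it.
; At zero, a DoOnce-guarded EndGame shows the cursor, switches input to UI only and passes both tallies to the widget's SwitchPanel.
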(event Custom|EndGame
  (bind _returnvalue (Game|GetPlayerController 0))
  (bind _widgettimer (Variables|Default|GetWidgetTimer))
  (Utilities|FlowControl|DoOnce false
    (:Completed
      ;[1 1 1] Wid
      (Variables|/Script/Engine.PlayerController|SetbShowMouseCursor _returnvalue true)
      (Input|SetInputModeUIOnly _returnvalue _widgettimer "DoNotLock" false)
      (Default|SwitchPanel _widgettimer (Variables|Default|GetNbSatisfied) (Variables|Default|GetNbUnsatisfied)))))

(event EventBeginPlay
  (Variables|Default|SetCurrentTimeGame (Variables|Default|GetDurationGame))
  (bind _returnvalue (UserInterface|CreateWidget "/Game/Widgets/WBP_EndGame.WBP_EndGame_C"))
  (bind _output_get (Variables|Default|SetWidgetTimer _returnvalue))
  (UserInterface|Viewport|AddtoViewport _output_get 0))

(event EventIncreaseSatisfied
  (Math|Integer|IncrementInt (Variables|Default|GetNbSatisfied)))

(event EventIncreaseUnsatisfied
  (Math|Integer|IncrementInt (Variables|Default|GetNbUnsatisfied)))

(event EventTick
  (params (DeltaSeconds :type Float%20%28single-precision%29))
  (bind _result (Math|Float|DecrementFloat (Variables|Default|GetCurrentTimeGame))
    (:%20%20
      (Default|SetTimer (Variables|Default|GetWidgetTimer) _result)
      (if (<= _result 0.0)
        (CallFunction|EndGame)))))

(fn ConstructionScript)